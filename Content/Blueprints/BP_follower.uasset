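; BP_follower is an actor that follows the player character.
; Each Tick it measures the distance to player 0, and while that is at least 100 units it moves toward the player along the normalized direction at a fixed speed scaled by DeltaSeconds.
; Movement uses a swept world offset rather than navigation or a movement component, and the construction script is empty.
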(event EventTick
  (params (DeltaSeconds :type Float%20%28single-precision%29))
  (bind _returnvalue (Game|GetPlayerCharacter 0))
  (bind _returnvalue_2 (Transformation|GetActorLocation))
  (bind _returnvalue_3 (Transformation|GetActorLocation _returnvalue))
  (if (>= (Math|Vector|Distance(Vector) _returnvalue_3 _returnvalue_2) 1e+02)
    (Transformation|AddActorWorldOffset (* DeltaSeconds (* (Math|Vector|Normalize (- _returnvalue_3 _returnvalue_2)) 1e+02)) true)))

(fn ConstructionScript)