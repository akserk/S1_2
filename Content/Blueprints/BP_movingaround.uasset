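; BP_movingaround is a Blueprint that moves its Cube component in a horizontal circle around its parent's origin.
; Each Tick adds delta time to Angle, then sets the cube's relative location from the cosine and sine of Angle scaled by Radius, at a fixed height.
; The RotateVector step uses a zero rotation, so it leaves the offset unchanged, and the move does not sweep for collision.
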(event EventTick
  (params (DeltaSeconds :type Float%20%28single-precision%29))
  (Variables|Default|Setangle (+ DeltaSeconds (Variables|Default|Getangle)))
  (Transformation|SetRelativeLocation (Variables|Default|GetCube) (Math|Vector|RotateVector (Math|Vector|MakeVector (* (Variables|Default|Getradius) (Math|Trig|Cos(Radians) (Variables|Default|Getangle))) (* (Variables|Default|Getradius) (Math|Trig|Sin(Radians) (Variables|Default|Getangle))) 5e+01) "0, 0, 0") false false))

(fn ConstructionScript)