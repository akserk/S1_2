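; Pufferfish actor that inflates as the third-person player character approaches it and shrinks back as the player moves away.
; Each tick it measures the distance to player 0's character, inverts it within a fixed radius and clamps the result into a uniform actor scale between normal and five times size.
; The scale follows distance directly, with no interpolation, and updates only while the player pawn is a BP_ThirdPersonCharacter.
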(event EventTick
  (params (DeltaSeconds :type Float%20%28single-precision%29))
  (bind _asbp_third_person_character (Utilities|Casting|CastToBP_ThirdPersonCharacter (Game|GetPlayerCharacter 0)))
  (Transformation|SetActorScale3D (Math|Conversions|ToVector(Float) (Math|Float|Clamp(Float) (/ (- 2.5e+02 (Math|Float|Clamp(Float) (Math|Vector|VectorLength (- (Transformation|GetActorLocation) (Transformation|GetActorLocation _asbp_third_person_character))) 0.0 2.5e+02)) 15.0) 1.0 5.0))))

(fn ConstructionScript)